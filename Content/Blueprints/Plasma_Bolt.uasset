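; Plasma bolt actor that destroys asteroids it overlaps and scores a point for the player's spaceship.
; On overlap with an Asteriod, it spawns an explosion, increments PlayerPoints on the Hero_Spaceship found by class lookup, then destroys the asteroid and itself.
; A Fire graph handles the Shoot input inside the bolt, disabling its own collision and spawning another Plasma_Bolt at its transform.
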(event EventBeginPlay
  (|CallParentFunction) ; This node is disabled and will not be called.\nDrag off pins to build functionality.
)

(event EventTick
  (params (DeltaSeconds :type Float%20%28single-precision%29))
  (|CallParentFunction DeltaSeconds) ; This node is disabled and will not be called.\nDrag off pins to build functionality.
)

(event Collision|EventActorBeginOverlap
  (params (OtherActor :type Actor%20Object%20Reference))
  (bind _asasteriod (Utilities|Casting|CastToAsteriod OtherActor))
  (Effects|SpawnEmitteratLocation "/Game/StarterContent/Particles/P_Explosion.P_Explosion" (Transformation|GetActorLocation))
  (bind _returnvalue (Actor|GetActorOfClass "/Game/Blueprints/Hero_Spaceship.Hero_Spaceship_C"))
  (Variables|/Game/Blueprints/Hero_Spaceship.Hero_Spaceship_C|SetPlayerPoints _returnvalue (+ (Variables|/Game/Blueprints/Hero_Spaceship.Hero_Spaceship_C|GetPlayerPoints _returnvalue) 1))
  (Actor|DestroyActor _asasteriod)
  (Actor|DestroyActor))

(event Input|ActionEvents|InputActionShoot
  (params (Key :type Key%20Structure))
  (:Pressed
    (Collision|SetActorEnableCollision false)
    (Game|SpawnActorfromClass "Plasma_Bolt_C" (Transformation|GetActorTransform) "Undefined" 0 0)))

(fn ConstructionScript
  (|CallParentFunction))